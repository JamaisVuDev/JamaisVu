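; Inverter gate Blueprint that acts as a logical NOT between an input Indicator and the objects wired to its outputs.
; Every Tick it reads the input's IsActivated state and loops over the Output array, applying the opposite state to each element.
; A chain of casts handles Indicators, glass doors and key stands through Activate/Deactivate, and goals through Enable/Disable.
; The state is polled and reapplied every frame, with no change detection.
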(event `self.ReceiveTick`
  (params (DeltaSeconds :type "Float (single-precision)"))
  (bind _asindicator (cast `/Game/Blueprints/Indicator` (`self.Input`)))
  (for _array_element (`self.Output`)
    (bind _asindicator_2 (cast `/Game/Blueprints/Indicator` _array_element)
      (:`then`
        (bind _returnvalue (not (`/Game/Blueprints/Indicator.isActivated` _asindicator)))
        (if _returnvalue
          (`/Game/Blueprints/Indicator.Activate` _asindicator_2)
          (else
            (`/Game/Blueprints/Indicator.Deactivate` _asindicator_2))))
      (:`CastFailed`
        (bind _asglass_door (cast `/Game/Blueprints/GlassDoor` _array_element)
          (:`then`
            (if _returnvalue
              (`/Game/Blueprints/GlassDoor.Activate` _asglass_door)
              (else
                (`/Game/Blueprints/GlassDoor.Deactivate` _asglass_door))))
          (:`CastFailed`
            (bind _askey_stand (cast `/Game/Blueprints/keyStand` _array_element)
              (:`then`
                (if _returnvalue
                  (`/Game/Blueprints/keyStand.Activate` _askey_stand)
                  (else
                    (`/Game/Blueprints/keyStand.Deactivate` _askey_stand))))
              (:`CastFailed`
                (bind _asgoal (cast `/Game/Blueprints/goal` _array_element))
                (if _returnvalue
                  (`/Game/Blueprints/goal.Enable` _asgoal)
                  (else
                    (`/Game/Blueprints/goal.Disable` _asgoal)))))))))))

(fn `UserConstructionScript`)