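; Goal actor that flags when the player can win by teleporting from it.
; Each tick it measures distance to the first MyCharacter, setting CanWin and drawing a "Press E to teleport" debug prompt when close, and clearing the flag otherwise.
; TurnSwitchOn and TurnSwitchOff each make opposite visibility calls to show the switch state; neither is called within this graph, nor is the E input handled here.
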(event `self.ReceiveTick`
  (params (DeltaSeconds :type "Float (single-precision)"))
  (bind _outactors (`GameplayStatics.GetAllActorsOfClass` null "/Game/Blueprints/MyCharacter.MyCharacter_C"))
  (bind _returnvalue (`self.GetDistanceTo` (`KismetArrayLibrary.Array_Get` _outactors)))
  (if (< _returnvalue 200.0)
    (set `self.canWin` true)
    (`KismetSystemLibrary.DrawDebugString` null (`self.K2_GetActorLocation`) "Press E to teleport" null (struct :`B` 1.0 :`A` 1.0))
    (else
      (set `self.canWin` false))))

(fn `Turn Switch Off`
  (`SceneComponent.SetVisibility` false)
  (`SceneComponent.SetVisibility` true))

(fn `turnSwitchOn`
  (`SceneComponent.SetVisibility` true)
  (`SceneComponent.SetVisibility` false))

(fn `UserConstructionScript`)