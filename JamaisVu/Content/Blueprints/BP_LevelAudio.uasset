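; BP_LevelAudio is a level audio actor that starts the level's background ambient sound on BeginPlay, if one is assigned.
; Pre-level narration logic, which attaches a sound to the MyCharacter actor and stores it in PreNarration, is disconnected along with its delay and never runs.
; StopPreLevelNarration stops that stored component, which nothing in the live graph sets.
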(event `self.ReceiveBeginPlay`
  (bind _backgroundsound (`self.BackgroundSound`))
  ;[1 1 1] If an ambient sound has been selected, play it at the start of the level
  (if (!= (`AudioComponent.Sound` _backgroundsound) null)
    (`AudioComponent.Play` _backgroundsound 0.0)))

(fn `StopPreLevelNarration`
  (`AudioComponent.Stop` (`self.PreNarration`)))

(fn `UserConstructionScript`)