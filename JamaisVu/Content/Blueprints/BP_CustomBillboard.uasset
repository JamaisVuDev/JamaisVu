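; BP_CustomBillboard is a billboard actor that appears when the player comes near and disappears for good once they leave.
; The construction script applies a configurable material, and BeginPlay sets initial visibility and caches the first MyCharacter found.
; Tick polls distance to that character, showing the billboard within a fixed radius and hiding it on exit.
; Two latching flags make this a one-shot cycle, after which distance checks stop.
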(event `self.ReceiveBeginPlay`
  (bind _outactors (`GameplayStatics.GetAllActorsOfClass` "/Game/Blueprints/MyCharacter.MyCharacter_C"))
  (set `self.PlayerRef` (`KismetArrayLibrary.Array_Get` _outactors))
  (`SceneComponent.SetVisibility` (`self.BillboardObject`) (`self.StartVisible`) false))

(event `self.ReceiveTick`
  (params (DeltaSeconds :type "Float (single-precision)"))
  (if (not (and (`self.playerHasEnteredRange`) (`self.playerHasLeftRange`)))
    (bind _returnvalue (`self.GetDistanceTo` (`self.PlayerRef`)))
    (if (< _returnvalue 1000.0)
      (set `self.playerHasEnteredRange` true)
      (`SceneComponent.SetVisibility` (`self.BillboardObject`) true false)
      (elif (`self.playerHasEnteredRange`)
        (set `self.playerHasLeftRange` true)
        (`SceneComponent.SetVisibility` (`self.BillboardObject`) false false)))))

(fn `UserConstructionScript`
  (`PrimitiveComponent.SetMaterial` (`self.BillboardObject`) 0 (`self.BillboardMaterial`)))