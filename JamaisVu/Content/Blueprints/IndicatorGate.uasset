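; IndicatorGate is an AND gate that powers puzzle elements when all of its linked input indicators are activated.
; Every Tick it polls the Inputs array, then switches everything in Outputs on or off to match, re-sending the call each frame.
; A cast chain picks the matching on/off call for Indicator, GlassDoor, keyStand or goal outputs, so gates can chain through Indicators.
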(event `self.ReceiveTick`
  (params (DeltaSeconds :type "Float (single-precision)"))
  (bind _outputs (`self.Outputs`))
  (set `self.allActivated` true)
  (for _array_element (`self.Inputs`)
    (bind _asindicator (cast `/Game/Blueprints/Indicator` _array_element))
    (if (not (`/Game/Blueprints/Indicator.isActivated` _asindicator))
      (set `self.allActivated` false)))
  (if (`self.allActivated`)
    (for _array_element_2 _outputs
      (bind _asindicator_2 (cast `/Game/Blueprints/Indicator` _array_element_2)
        (:`then`
          (`/Game/Blueprints/Indicator.Activate` _asindicator_2))
        (:`CastFailed`
          (bind _asglass_door (cast `/Game/Blueprints/GlassDoor` _array_element_2)
            (:`then`
              (`/Game/Blueprints/GlassDoor.PowerOn` _asglass_door))
            (:`CastFailed`
              (bind _askey_stand (cast `/Game/Blueprints/keyStand` _array_element_2)
                (:`then`
                  (`/Game/Blueprints/keyStand.Activate` _askey_stand))
                (:`CastFailed`
                  (bind _asgoal (cast `/Game/Blueprints/goal` _array_element_2))
                  (`/Game/Blueprints/goal.Enable` _asgoal))))))))
    (else
      (for _array_element_3 _outputs
        (bind _asindicator_3 (cast `/Game/Blueprints/Indicator` _array_element_3)
          (:`then`
            (`/Game/Blueprints/Indicator.Deactivate` _asindicator_3))
          (:`CastFailed`
            (bind _asglass_door_2 (cast `/Game/Blueprints/GlassDoor` _array_element_3)
              (:`then`
                (`/Game/Blueprints/GlassDoor.PowerOff` _asglass_door_2))
              (:`CastFailed`
                (bind _askey_stand_2 (cast `/Game/Blueprints/keyStand` _array_element_3)
                  (:`then`
                    (`/Game/Blueprints/keyStand.Deactivate` _askey_stand_2))
                  (:`CastFailed`
                    (bind _asgoal_2 (cast `/Game/Blueprints/goal` _array_element_3))
                    (`/Game/Blueprints/goal.Disable` _asgoal_2)))))))))))

(fn `UserConstructionScript`)