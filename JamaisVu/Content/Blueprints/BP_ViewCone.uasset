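; View cone actor that traces the shape of a cone clipped by world geometry and shows it with debug lines.
; Each tick, DrawViewCone line-traces a ring of directions around its forward axis and rebuilds a list of double-sided triangles.
; Tick draws red lines to those vertices and a white forward line.
; Mesh upload, edge stitching and beam updates are disconnected, so the triangles never reach ConeMesh and the spawned beam emitters stay unaimed.
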(event EventBeginPlay
  (Rendering|Material|SetMaterial (Variables|Default|GetConeMesh) 0 "/Game/Character/mat_cone.mat_cone")
  (Variables|Default|Setsegments 32)
  (Variables|Default|SetdegreeIncrement (/ 3.6e+02 (Math|Conversions|ToFloat(Integer) (Variables|Default|Getsegments))))
  (Variables|Default|SetconeHalfAngle 4e+01)
  (for _index (range 0 (- (Variables|Default|Getsegments) 1))
    (bind _returnvalue (Effects|SpawnEmitterAttached "/Game/Blueprints/beam_particle.beam_particle" (Variables|Default|GetConeMesh) "None" "0, 0,0.000000" "0.000000, 0,0.000000" "KeepWorldPosition"))
    (Utilities|Array|Add (Variables|Default|GetEmitterList) _returnvalue)))

(event EventTick
  (params (DeltaSeconds :type Float%20%28single-precision%29))
  (bind _returnvalue (Transformation|GetWorldTransform))
  (bind _coneendpoint (Variables|Default|GetconeEndpoint))
  (bind _coneendpoint_2 (Variables|Default|GetconeEndpoint))
  (bind (_location _rotation) (Math|Transform|BreakTransform _returnvalue))
  (Variables|Default|SetdegreeIncrement (/ 3.6e+02 (Math|Conversions|ToFloat(Integer) (Variables|Default|Getsegments))))
  (CallFunction|DrawViewCone _location _rotation)
  (for (_array_element _array_index) (Variables|Default|GetcustomMeshTriangleList)
    (if (== (Math|Integer|%(Integer) _array_index 2) 1)
      (Rendering|Debug|DrawDebugLine _coneendpoint (+ _coneendpoint (.Vertex1 (Utilities|Struct|BreakCustomMeshTriangle _array_element))) "(R=1.000000,G=0.000000,B=0.000000,A=1.000000)" 0.0 2.0)
      (Rendering|Debug|DrawDebugLine _coneendpoint_2 (+ _coneendpoint_2 (* (Math|Vector|Normalize (Variables|Default|GetlocalForward)) 5e+03)) "(R=1.000000,G=1.000000,B=1.000000,A=1.000000)" 0.0 5.0))))

(fn ConstructionScript)

(fn AddConeGeometry
  (params (Theta :type Float%20%28single-precision%29))
  (bind _vectorfromendpoint (Util|GetVertexDirection (+ Theta (Variables|Default|GetdegreeIncrement))))
  (LocalVariables|SetVector1 _vectorfromendpoint)
  (bind _vectorfromendpoint_2 (Util|GetVertexDirection Theta))
  (LocalVariables|SetVector2 _vectorfromendpoint_2)
  ;[1 1 1] Add standard cone triangle
  (bind _trianglevertex (CallFunction|RaycasttoWall (LocalVariables|GetVector1) (Variables|Default|GetconeEndpoint)))
  (LocalVariables|SetVert1 _trianglevertex)
  (bind _trianglevertex_2 (CallFunction|RaycasttoWall (LocalVariables|GetVector2) (Variables|Default|GetconeEndpoint)))
  (LocalVariables|SetVert2 _trianglevertex_2)
  (CallFunction|AddTriangletoList "0, 0,0.000000" (LocalVariables|GetVert1) (LocalVariables|GetVert2) true))

(fn DrawViewCone
  (params (endpoint :type Vector) (coneRotation :type Rotator))
  (Variables|Default|SetconeEndpoint endpoint)
  (Variables|Default|SetconeRotator coneRotation)
  (Variables|Default|SetlocalForward (Math|Vector|RotateVector "1.000000, 0,0.000000" coneRotation))
  (Variables|Default|SetlocalUp (Math|Vector|RotateVector "0.000000, 0,1.000000" coneRotation))
  (Variables|Default|SetlocalRight (Math|Vector|CrossProduct (Variables|Default|GetlocalForward) (Variables|Default|GetlocalUp)))
  (Utilities|Array|Clear (Variables|Default|GetcustomMeshTriangleList))
  (for _index (range 0 (- (Variables|Default|Getsegments) 1))
    (CallFunction|AddConeGeometry (* _index (Variables|Default|GetdegreeIncrement)))))

(fn GetVertexDirection
  (params (Theta :type Float%20%28single-precision%29))
  (bind _conehalfangle (Variables|Default|GetconeHalfAngle))
  (bind _returnvalue (Math|Trig|Tan(Degrees) _conehalfangle))
  (return (+ (Variables|Default|GetlocalForward) (* (* (Variables|Default|GetlocalRight) (Math|Trig|Cos(Degrees) Theta)) _returnvalue) (* (* (Variables|Default|GetlocalUp) (Math|Trig|Sin(Degrees) Theta)) _returnvalue))))

(fn RaycasttoWall
  (params (DirectionVector :type Vector) (StartLocation :type Vector))
  (bind _returnvalue (Math|Vector|Normalize DirectionVector))
  (bind _returnvalue_2 (* _returnvalue 1e+04))
  ;[1 1 1] Returns vertex in local space
  (LocalVariables|SetStartPoint StartLocation)
  (bind (_outhit _returnvalue_3) (Collision|LineTraceForObjects (LocalVariables|GetStartPoint) (+ (LocalVariables|GetStartPoint) _returnvalue_2) (Utilities|Array|MakeArray "ObjectTypeQuery2" "ObjectTypeQuery1") false 0 "None"))
  (if _returnvalue_3
    (Utilities|IsValid (.HitActor (Collision|BreakHitResult _outhit))
      (:Is%20Valid
        (LocalVariables|SethitLocation (- (.Location (Collision|BreakHitResult _outhit)) (LocalVariables|GetStartPoint))))
      (:Is%20Not%20Valid
        (LocalVariables|SethitLocation (- _returnvalue_2 (LocalVariables|GetStartPoint)) :!label _label)))
    (else
      (goto _label)))
  (return (LocalVariables|GethitLocation)))

(fn AddTriangletoList
  (params (Point0 :type Vector) (Point1 :type Vector) (Point2 :type Vector) (doubleSided :type Boolean))
  ;[1 1 1] Add a triangle to the list
  (Utilities|Array|Add (Variables|Default|GetcustomMeshTriangleList) (Utilities|Struct|MakeCustomMeshTriangle Point0 Point1 Point2))
  ;[1 1 1] Add a triangle with the opposite normal as well, if set
  (if doubleSided
    (Utilities|Array|Add (Variables|Default|GetcustomMeshTriangleList) (Utilities|Struct|MakeCustomMeshTriangle Point0 Point2 Point1))))

(fn RaycastinDirecction
  (params (DirectionVector :type Vector) (StartLocation :type Vector))
  (bind _returnvalue (Math|Vector|Normalize DirectionVector))
  (bind _returnvalue_2 (* _returnvalue 1e+04))
  ;[1 1 1] Returns vertex in world space
  (LocalVariables|SetStartPoint StartLocation)
  (bind (_outhit _returnvalue_3) (Collision|LineTraceForObjects (LocalVariables|GetStartPoint) (+ (LocalVariables|GetStartPoint) _returnvalue_2) (Utilities|Array|MakeArray "ObjectTypeQuery2" "ObjectTypeQuery1") false 0 "None"))
  (if _returnvalue_3
    (Utilities|IsValid (.HitActor (Collision|BreakHitResult _outhit))
      (:Is%20Valid
        (LocalVariables|SethitLocation (- (.Location (Collision|BreakHitResult _outhit)) "0, 0, 0")))
      (:Is%20Not%20Valid
        (LocalVariables|SethitLocation (- _returnvalue_2 "0, 0, 0") :!label _label)))
    (else
      (goto _label)))
  (return (LocalVariables|GethitLocation)))

(fn GetAngleBetweenVectors
  (params (Vector1 :type Vector) (Vector2 :type Vector))
  (return (Class|KismetMathLibrary|DegAcos (/ (Math|Vector|DotProduct Vector1 Vector2) (* (Math|Vector|VectorLength Vector1) (Math|Vector|VectorLength Vector2))))))

(fn Between
  (params (Value :type Float%20%28single-precision%29) (Min :type Float%20%28single-precision%29) (Max :type Float%20%28single-precision%29))
  (return (and (>= Value Min) (<= Value Max))))

(fn InRangeOf
  (params (Value1 :type Float%20%28single-precision%29) (Value2 :type Float%20%28single-precision%29) (Distance :type Float%20%28single-precision%29))
  (return (<= (Math|Float|Absolute(Float) (- Value1 Value2)) (Math|Float|Absolute(Float) Distance))))