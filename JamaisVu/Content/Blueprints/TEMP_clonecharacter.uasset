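; A temporary clone character Blueprint containing a prototype view-cone check for detecting the player, currently disconnected.
; The unwired ConeCheck logic reads a look direction from LookList at TransformIndex to set the cone's pitch, remapped to a narrower range.
; It flags the player as within the cone by comparing the dot-product angle against a threshold, with no distance test, and shows debug text.
; Both the construction script and ConeCheck are empty as wired.
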(fn `ConeCheck`)

(fn `UserConstructionScript`)