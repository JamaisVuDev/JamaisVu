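; A clock Blueprint that shows a looping seconds countdown on its TimerText, or a blinking zero display when no positive LoopTime is set.
; Tick counts TimeLeft down by delta time and restarts it on expiry, carrying the overshoot into the next cycle.
; The countdown shows rounded-up seconds, zero-padded below ten, with minutes fixed at zero.
; Without a loop time, the same timer toggles BlinkOn each second to alternate "0:00" and empty text.
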(event `self.ReceiveBeginPlay`
  ;[1 1 1] Check if the clock has a positive loop time
  (if (> (`self.loopTime`) 0.0)
    (set `self.timeLeft` (`self.loopTime`))
    (else
      (set `self.timeLeft` 1.0))))

(event `self.ReceiveTick`
  (params (DeltaSeconds :type "Float (single-precision)"))
  (bind _timertext (`self.TimerText`))
  (bind _returnvalue (`KismetMathLibrary.FCeil` (`self.timeLeft`)))
  ;[1 1 1] Check if the clock has a positive loop time
  (if (> (`self.loopTime`) 0.0)
    (if (<= (`self.timeLeft`) 0.0)
      ;[1 1 1] When the timer runs out, reset it
      (set `self.timeLeft` (- (`self.loopTime`) (- 0.0 (`self.timeLeft`))))
      (else
        ;[1 1 1] Decrement time left
        (set `self.timeLeft` (- (`self.timeLeft`) DeltaSeconds))))
    (if (< _returnvalue 10)
      ;[1 1 1] If time left is less than 10 seconds, add a 0 in front of the value
      (`TextRenderComponent.SetText` (`self.TimerText`) (`KismetStringLibrary.Concat_StrStr` "0:0" (`KismetStringLibrary.Conv_IntToString` _returnvalue)))
      (else
        ;[1 1 1] If time left is greater than 10 seconds, display the value
        (`TextRenderComponent.SetText` (`self.TimerText`) (`KismetStringLibrary.Concat_StrStr` "0:" (`KismetStringLibrary.Conv_IntToString` _returnvalue)))))
    (elif (<= (`self.timeLeft`) 0.0)
      ;[1 1 1] If the time is below 0, toggle blinking and change text
      (set `self.timeLeft` (- 1.0 (- 0.0 (`self.timeLeft`))))
      (set `self.blinkOn` (not (`self.blinkOn`)))
      (if (`self.blinkOn`)
        (`TextRenderComponent.SetText` _timertext "0:00")
        (else
          (`TextRenderComponent.SetText` _timertext "     ")))
      (else
        ;[1 1 1] Decrement time left
        (set `self.timeLeft` (- (`self.timeLeft`) DeltaSeconds))))))

(fn `UserConstructionScript`)