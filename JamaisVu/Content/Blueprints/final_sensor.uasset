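; Final sensor pressure-plate actor that enables its linked goal objects when the player's remaining time is about ten seconds.
; Tick polls TimeLeft on the first MyCharacter found at BeginPlay and calls ActivateAll on every tick within a small tolerance window.
; The construction script derives a scaled radius and picks a red or green material.
; DeactivateAll and the radius-and-height CheckInRange test are defined but not called here.
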(event EventTick
  (params (DeltaSeconds :type Float%20%28single-precision%29))
  ;[1 1 1] If sensor was activated, call activate once (until deactivated)
  (if (Math|Float|NearlyEqual(Float) (Variables|/Game/Blueprints/MyCharacter.MyCharacter_C|GettimeLeft (Variables|Default|Getplayer_ref)) 1e+01 0.1)
    (CallFunction|ActivateAll)))

(event EventBeginPlay
  (bind _outactors (Actor|GetAllActorsOfClass 0 "/Game/Blueprints/MyCharacter.MyCharacter_C"))
  (Variables|Default|Setplayer_ref (Utilities|Array|Get(acopy) _outactors)))

(fn ConstructionScript
  (bind _returnvalue (Transformation|GetActorTransform))
  (bind _pressureplate (Variables|Default|GetPressurePlate))
  (bind _scale (Math|Transform|BreakTransform _returnvalue))
  (bind (_x _y) (Math|Vector|BreakVector _scale))
  (Variables|Default|SetcapsuleRadius (* (Variables|/Script/Engine.CapsuleComponent|GetCapsuleRadius (Variables|Default|GetCollisionComponent)) (/ (+ _x _y) 2.0)))
  ;[1 1 1] Set the sensor material based on its function
  (if (Variables|Default|GetPositionOrKey)
    (Rendering|Material|SetMaterial _pressureplate 1 "/Game/Materials/SensorRedMaterial.SensorRedMaterial")
    (else
      (Rendering|Material|SetMaterial _pressureplate 1 "/Game/Materials/SensorGreenMaterial.SensorGreenMaterial"))))

(fn DeactivateAll
  ;[1 1 1] Deactivate all attached objects
  (for _array_element (Variables|ActivableObjects|GetactivableObjects)
    (bind _asgoal (Utilities|Casting|CastTogoal _array_element))
    (Default|Disable _asgoal)))

(fn ActivateAll
  ;[1 1 1] Deactivate all attached objects
  (for _array_element (Variables|ActivableObjects|GetactivableObjects)
    (bind _asgoal (Utilities|Casting|CastTogoal _array_element))
    (Default|Enable _asgoal)))

(fn CheckinRange
  (params (OtherObject :type Actor%20Object%20Reference) (objectType :type Byte))
  (bind _returnvalue (Transformation|GetActorLocation OtherObject))
  (bind _returnvalue_2 (Transformation|GetActorLocation))
  (bind _returnvalue_3 (- _returnvalue _returnvalue_2))
  (bind (_x _y _z) (Math|Vector|BreakVector _returnvalue_3))
  (bind _returnvalue_4 (Math|Float|Absolute(Float) _z))
  ;[1 1 1] Return whether or not object is within range of the pressure plate
  (switch int (Math|Conversions|ToInteger(Byte) objectType)
    (:Default
      (LocalVariables|SetotherObjectRadius 1e+02 :!label _label)
      (if (and (< (Math|Vector|VectorLength (Math|Vector|MakeVector _x _y 0.0)) (+ (Variables|Default|GetcapsuleRadius) (LocalVariables|GetotherObjectRadius))) (< _returnvalue_4 108.0))
        (LocalVariables|SetisObjectInRange true :!label _label_2)
        (else
          (LocalVariables|SetisObjectInRange false :!label _label_3))))
    (:0
      (goto _label))
    (:1
      (LocalVariables|SetotherObjectRadius 8e+01)
      (if (and (< (Math|Vector|VectorLength (Math|Vector|MakeVector _x _y 0.0)) (+ (Variables|Default|GetcapsuleRadius) (LocalVariables|GetotherObjectRadius))) (< _returnvalue_4 5e+01))
        (goto _label_2)
        (else
          (goto _label_3))))
    (:2
      (goto _label)))
  (return (LocalVariables|GetisObjectInRange)))