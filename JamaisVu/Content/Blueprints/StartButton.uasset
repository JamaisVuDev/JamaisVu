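; StartButton is an in-world button actor that the player can use to begin the level.
; Until the level has begun, each Tick sets CanBegin by the first MyCharacter's proximity and draws a "Press E to begin." debug string above the button, regardless of distance.
; TurnButtonOn clears CanBegin and sets LevelBegun, stopping the check and prompt; input handling is not in this Blueprint.
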(event `self.ReceiveTick`
  (params (DeltaSeconds :type "Float (single-precision)"))
  (if (not (`self.LevelBegun`))
    (bind _outactors (`GameplayStatics.GetAllActorsOfClass` null "/Game/Blueprints/MyCharacter.MyCharacter_C"))
    (bind _returnvalue (`self.GetDistanceTo` (`KismetArrayLibrary.Array_Get` _outactors)))
    (if (< _returnvalue 300.0)
      (set `self.CanBegin` true)
      (else
        (set `self.CanBegin` false)))
    (`KismetSystemLibrary.DrawDebugString` null (+ (`self.K2_GetActorLocation`) (0.0 0.0 30.0)) "Press E to begin." null (struct :`B` 1.0 :`A` 1.0))))

(fn `Turn Button On`
  (set `self.CanBegin` false)
  (set `self.LevelBegun` true))

(fn `UserConstructionScript`)