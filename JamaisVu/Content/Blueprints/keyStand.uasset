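; Key stand with a glass cover that lowers on Activate and rises on Deactivate, driven by a timeline playing forward and in reverse.
; StartDown places the glass open or closed in the construction script; when set, the stand ignores all three events, apart from Resetstand's debug print.
; Resetstand otherwise resets the timeline's time.
; Older logic that polls and XORs Indicator inputs remains in the graph but is disconnected.
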(event `Activate`
  ;[1 1 1] If not set to start down, move the glass when input is received
  (if (not (`self.startDown`))
    (bind (_direction _glassposition) (`Timeline|Timeline_open` :`NewTime` 1.0 :!label _label)
      (:`Update`
        (`SceneComponent.K2_SetRelativeLocation` (`self.keyStandGlass`) _glassposition false)))))

(event `Deactivate`
  ;[1 1 1] If not set to start down, move the glass when input is received
  (if (not (`self.startDown`))
    (goto _label :!via `Reverse`)))

(event `Reset stand`
  ;[1 1 1] If not set to start down, move the glass when input is received
  (`KismetSystemLibrary.PrintString` null "RESETTING STAND" true true (struct :`G` 0.66 :`B` 1.0))
  (if (not (`self.startDown`))
    (goto _label :!via `SetNewTime`)))

(event `self.ReceiveTick`
  (params (DeltaSeconds :type "Float (single-precision)")))

(fn `UserConstructionScript`
  (if (`self.startDown`)
    ;[1 1 1] If set to start down, set glass to the open position
    (`SceneComponent.K2_SetRelativeLocation` (`self.keyStandGlass`) (`KismetMathLibrary.MakeVector` 0.0 0.0 -175.0) false)
    (else
      ;[1 1 1] If set to start down, set glass to the closed position
      (`SceneComponent.K2_SetRelativeLocation` (`self.keyStandGlass`) (`KismetMathLibrary.MakeVector` 0.0) false))))