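; Pressure plate sensor that powers its linked GlassDoor and Indicator actors while a player character, Key or clone is on it.
; Tick polls those actors using per-type horizontal and height distance checks, requiring floor-level placement at Z scale 1.
; Two DoOnce nodes form an SR latch, so power and plate material switch only on state changes.
; Construction derives detection radius from XY scale and picks red or green material from PositionOrKey.
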(event EventTick
  (params (DeltaSeconds :type Float%20%28single-precision%29))
  ;[1 1 1] Check whether the sensor should be activated, and toggle its state accordingly.      IMPORTANT: In order for this to work, sensor must be placed at the same Z value as the floor object, and at a Z scale of 1.
  (Variables|Default|SetactivatedThisFrame false)
  ;;[0.568 0.4874 1] Check if the player is standing on the pressure plate
  (bind _outactors (Actor|GetAllActorsOfClass "/Game/Blueprints/MyCharacter.MyCharacter_C"))
  (for _array_element _outactors
    ;;;[1 1 1] If activated, no longer check
    (if (not (Variables|Default|GetactivatedThisFrame))
      (bind _objectinrange (CallFunction|CheckinRange _array_element))
      (if _objectinrange
        ;;[1 1 1] If sensor was activated, call activate once (until deactivated)
        (Variables|Default|SetactivatedThisFrame true)
        ;;[1 1 1] SR latch for activation (to ensure state can only toggle based on proximity)
        (Utilities|FlowControl|DoOnce false
          (:Completed
            (Variables|Default|SetobjectInRange true)
            (CallFunction|ActivateAll)
            (goto _label Reset))))))
  ;;[0.441 1 0.5605] Check if there is a key on the pressure plate
  (bind _outactors_2 (Actor|GetAllActorsOfClass "/Game/Blueprints/Key.Key_C"))
  (for _array_element_2 _outactors_2
    ;;;[1 1 1] If activated, no longer check
    (if (not (Variables|Default|GetactivatedThisFrame))
      (bind _objectinrange_2 (CallFunction|CheckinRange _array_element_2 1))
      (if _objectinrange_2
        (Variables|Default|SetactivatedThisFrame true)
        (Utilities|FlowControl|DoOnce false
          (:Completed
            (Variables|Default|SetobjectInRange true)
            (CallFunction|ActivateAll)
            (goto _label Reset))))))
  ;;[0.8017 0.4114 1] Check if any clones are on the pressure plate
  (bind _outactors_3 (Actor|GetAllActorsOfClass "/Game/Blueprints/BP_CloneCharacter.BP_CloneCharacter_C"))
  (for _array_element_3 _outactors_3
    ;;;[1 1 1] If activated, no longer check
    (if (not (Variables|Default|GetactivatedThisFrame))
      (bind _objectinrange_3 (CallFunction|CheckinRange _array_element_3 2))
      (if _objectinrange_3
        (Variables|Default|SetactivatedThisFrame true)
        (Utilities|FlowControl|DoOnce false
          (:Completed
            (Variables|Default|SetobjectInRange true)
            (CallFunction|ActivateAll)
            (goto _label Reset))))))
  ;;[1 1 1] If the sensor was not activated, call deactivate once (until activated)
  (if (not (Variables|Default|GetactivatedThisFrame))
    (Utilities|FlowControl|DoOnce true :!label _label
      (:Completed
        (Variables|Default|SetobjectInRange false)
        (CallFunction|DeactivateAll)
        (Utilities|FlowControl|DoOnce false) ; enters at Reset
      ))))

(fn ConstructionScript
  (bind _returnvalue (Transformation|GetActorTransform))
  (bind _pressureplate (Variables|Default|GetPressurePlate))
  (bind _scale (Math|Transform|BreakTransform _returnvalue))
  (bind (_x _y) (Math|Vector|BreakVector _scale))
  (Variables|Default|SetcapsuleRadius (* (Variables|/Script/Engine.CapsuleComponent|GetCapsuleRadius (Variables|Default|GetCollisionComponent)) (/ (+ _x _y) 2.0)))
  ;[1 1 1] Set the sensor material based on its function
  (if (Variables|Default|GetPositionOrKey)
    (Rendering|Material|SetMaterial _pressureplate 1 "/Game/Materials/SensorRedMaterial.SensorRedMaterial")
    (else
      (Rendering|Material|SetMaterial _pressureplate 1 "/Game/Materials/SensorGreenMaterial.SensorGreenMaterial"))))

(fn DeactivateAll
  ;[1 1 1] Deactivate all attached objects
  (Rendering|Material|SetMaterial (Variables|Default|GetPressurePlate) 0 "/Game/Materials/SensorDisabledMaterial.SensorDisabledMaterial")
  (for _array_element (Variables|ActivableObjects|GetactivableObjects)
    (bind _asglass_door (Utilities|Casting|CastToGlassDoor _array_element)
      (:then
        (Default|PowerOff _asglass_door))
      (:CastFailed
        (bind _asindicator (Utilities|Casting|CastToIndicator _array_element))
        (Default|PowerOff _asindicator)))))

(fn ActivateAll
  ;[1 1 1] Deactivate all attached objects
  (Rendering|Material|SetMaterial (Variables|Default|GetPressurePlate) 0 "/Game/Materials/SensorEnabledMaterial.SensorEnabledMaterial")
  (for _array_element (Variables|ActivableObjects|GetactivableObjects)
    (bind _asglass_door (Utilities|Casting|CastToGlassDoor _array_element)
      (:then
        (Default|Poweron _asglass_door))
      (:CastFailed
        (bind _asindicator (Utilities|Casting|CastToIndicator _array_element))
        (Default|Poweron _asindicator)))))

(fn CheckinRange
  (params (OtherObject :type Actor%20Object%20Reference) (objectType :type Byte))
  (bind _returnvalue (Transformation|GetActorLocation OtherObject))
  (bind _returnvalue_2 (Transformation|GetActorLocation))
  (bind _returnvalue_3 (- _returnvalue _returnvalue_2))
  (bind (_x _y _z) (Math|Vector|BreakVector _returnvalue_3))
  (bind _returnvalue_4 (Math|Float|Absolute(Float) _z))
  ;[1 1 1] Return whether or not object is within range of the pressure plate
  (switch int (Math|Conversions|ToInteger(Byte) objectType)
    (:Default
      (LocalVariables|SetotherObjectRadius 1e+02 :!label _label)
      (if (and (< (Math|Vector|VectorLength (Math|Vector|MakeVector _x _y 0.0)) (+ (Variables|Default|GetcapsuleRadius) (LocalVariables|GetotherObjectRadius))) (< _returnvalue_4 108.0))
        (LocalVariables|SetisObjectInRange true :!label _label_2)
        (else
          (LocalVariables|SetisObjectInRange false :!label _label_3))))
    (:0
      (goto _label))
    (:1
      (LocalVariables|SetotherObjectRadius 8e+01)
      (if (and (< (Math|Vector|VectorLength (Math|Vector|MakeVector _x _y 0.0)) (+ (Variables|Default|GetcapsuleRadius) (LocalVariables|GetotherObjectRadius))) (< _returnvalue_4 5e+01))
        (goto _label_2)
        (else
          (goto _label_3))))
    (:2
      (goto _label)))
  (return (LocalVariables|GetisObjectInRange)))