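; Lightning bolt that periodically flashes a vertical beam particle with a thunder or strike sound, hidden on BeginPlay.
; StartTimer schedules the first strike; ShootLightning then shows the beam, replays the sound, reschedules itself by name and sets a short timer to hide the beam.
; StopTimer cancels the cycle and silences it, while an Active flag tracks when the bolt is visible.
; The delayed self-destroy chain in the event graph is disconnected.
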(event `self.ReceiveBeginPlay`
  (bind _lightningbolt (`self.LightningBolt`))
  (`SceneComponent.SetVisibility` (`self.LightningBolt`) false true)
  (`ParticleSystemComponent.SetBeamSourcePoint` _lightningbolt 0 (0.0 0.0 0.0) 0)
  (`ParticleSystemComponent.SetBeamTargetPoint` _lightningbolt 0 (0.0 0.0 10000.0) 0))

(fn `ShootLightning`
  (bind _lightningsound (`self.LightningSound`))
  (`SceneComponent.SetVisibility` (`self.LightningBolt`) true true)
  (set `self.Active` true)
  (`AudioComponent.Stop` _lightningsound)
  (`AudioComponent.Play` _lightningsound 0.0)
  (`KismetSystemLibrary.K2_SetTimer` null "ShootLightning" 25.0)
  (`KismetSystemLibrary.K2_SetTimer` null "StopLightning" 0.2))

(fn `StartTimer`
  (`AudioComponent.Stop` (`self.LightningSound`))
  (`SceneComponent.SetVisibility` (`self.LightningBolt`) false true)
  (set `self.Active` false)
  (`KismetSystemLibrary.K2_SetTimer` null "ShootLightning" 15.7))

(fn `StopLightning`
  (`SceneComponent.SetVisibility` (`self.LightningBolt`) false true)
  (set `self.Active` false))

(fn `StopTimer`
  (`self.StopLightning`)
  (`AudioComponent.Stop` (`self.LightningSound`))
  (set `self.Active` false)
  (`KismetSystemLibrary.K2_ClearTimer` null "ShootLightning"))

(fn `UserConstructionScript`)