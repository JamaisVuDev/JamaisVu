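; A powered glass door that opens while at least one power source feeds it and closes when none remain.
; PowerOn and PowerOff track the source count, driving a timeline that squashes and shifts the door aside and switching the frame's sensor between green and red.
; The construction script picks the transparent or alternate door material and optionally snaps the actor to a wall by line trace, aligning it to the hit normal.
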(event Custom|Activate
  (bind _doorobject (Variables|Default|GetdoorObject))
  (Rendering|Material|SetMaterial (Variables|Default|GetdoorFrame) 2 "/Game/Materials/SensorGreenMaterial.SensorGreenMaterial")
  (bind _door_offset (Timeline|DoorMove Play)
    (:Update
      (Transformation|SetRelativeScale3D _doorobject (Math|Vector|MakeVector (Math|Float|Lerp 1.0 0.2 (.Y (Math|Vector|BreakVector _door_offset))) 1.0 1.0))
      (Transformation|SetRelativeLocation _doorobject (Math|Vector|MakeVector (Math|Float|Lerp 0.0 -65.0 (.Y (Math|Vector|BreakVector _door_offset))) 0.0 0.0) false))))

(event Custom|Deactivate
  (bind _doorobject (Variables|Default|GetdoorObject))
  (Rendering|Material|SetMaterial (Variables|Default|GetdoorFrame) 2 "/Game/Materials/SensorRedMaterial.SensorRedMaterial")
  (bind _door_offset (Timeline|DoorMove Reverse)
    (:Update
      (Transformation|SetRelativeScale3D _doorobject (Math|Vector|MakeVector (Math|Float|Lerp 1.0 0.2 (.Y (Math|Vector|BreakVector _door_offset))) 1.0 1.0))
      (Transformation|SetRelativeLocation _doorobject (Math|Vector|MakeVector (Math|Float|Lerp 0.0 -65.0 (.Y (Math|Vector|BreakVector _door_offset))) 0.0 0.0) false))))

(fn ConstructionScript
  (if (Variables|Default|Gettransparent)
    (Rendering|Material|SetMaterial (Variables|Default|GetdoorObject) 0 "/Game/Maps/level_0-3+(1-1)/Door.Door")
    (else
      (Rendering|Material|SetMaterial (Variables|Default|GetdoorObject) 0 "/Game/Materials/DoorMaterial.DoorMaterial")))
  (if (Variables|LevelEditing|GetSnapToWall)
    (Rendering|SetVisibility (Variables|Default|GetArrowTowardsWall) true false)
    (Rendering|SetVisibility (Variables|Default|GetWallPlane) true false)
    (LevelEditing|SnaptoLevel)
    (else
      (Rendering|SetVisibility (Variables|Default|GetArrowTowardsWall) false false)
      (Rendering|SetVisibility (Variables|Default|GetWallPlane) false false))))

(fn Poweron
  (Variables|Default|SetpoweredSources (+ (Variables|Default|GetpoweredSources) 1))
  (CallFunction|Activate))

(fn PowerOff
  (Variables|Default|SetpoweredSources (Math|Integer|Clamp(Integer) (- (Variables|Default|GetpoweredSources) 1) 0 32))
  (if (== (Variables|Default|GetpoweredSources) 0)
    (CallFunction|Deactivate)))

(fn SnaptoLevel
  (LocalVariables|SetTowardsWall (* (Transformation|GetActorForwardVector) -1.0))
  (LocalVariables|SetCurrentLocation (+ (Transformation|GetWorldLocation (Variables|Default|GetFrameCenter)) (* (Math|Vector|Normalize (Transformation|GetActorForwardVector)) 4e+01)))
  (bind (_outhit _returnvalue) (Collision|LineTraceForObjects 0 (LocalVariables|GetCurrentLocation) (+ (LocalVariables|GetCurrentLocation) (* (Math|Vector|Normalize (LocalVariables|GetTowardsWall)) 1.6e+02)) (Utilities|Array|MakeArray "ObjectTypeQuery2" "ObjectTypeQuery1") false 0 "None"))
  (if _returnvalue
    (Utilities|IsValid (.HitActor (Collision|BreakHitResult _outhit))
      (:Is%20Valid
        ;[1 1 1] Translate and rotate this object to snap to the wall or floor underneath it
        (Transformation|SetActorLocation (+ (- (.Location (Collision|BreakHitResult _outhit)) (- (Transformation|GetWorldLocation (Variables|Default|GetFrameCenter)) (Transformation|GetActorLocation))) (* (Math|Vector|Normalize (* (.Normal (Collision|BreakHitResult _outhit)) 1.0)) 42.0)) false)
        (if (not (Math|Vector|Equal(Vector) (Math|Vector|Normalize (Math|Vector|GetUpVector (Math|Rotator|MakeRotfromZ (.Normal (Collision|BreakHitResult _outhit))))) (Math|Vector|Normalize (Transformation|GetActorForwardVector)) 0.001))
          (Transformation|SetActorRotation (Math|Rotator|MakeRotfromX (.Normal (Collision|BreakHitResult _outhit)))))))))