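; BP_Clock is a wall-mountable countdown clock that shows seconds on a text component.
; Tick blinks "0:00" each second until ResetTimer is called, then counts down from LoopTime and wraps around when it runs out.
; With SnapToWall enabled, the construction script shows the guide arrow and plane, then line-traces behind the actor to offset and align it to the surface hit.
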(event EventTick
  (params (DeltaSeconds :type Float%20%28single-precision%29))
  (bind _timertext (Variables|Default|GetTimerText))
  ;[1 1 1] Check if the clock has been started
  (if (Variables|Default|GethasStarted)
    (if (<= (Variables|Default|GettimeLeft) 0.0)
      ;[1 1 1] When the timer runs out, reset it
      (Variables|Default|SettimeLeft (- (Variables|Default|GetloopTime) (- 0.0 (Variables|Default|GettimeLeft))))
      (else
        ;[1 1 1] Decrement time left
        (Variables|Default|SettimeLeft (- (Variables|Default|GettimeLeft) DeltaSeconds))))
    (if (< (Math|Float|Ceil (Variables|Default|GettimeLeft)) 10)
      ;[1 1 1] If time left is less than 10 seconds, add a 0 in front of the value
      (Rendering|Components|TextRender|SetText (Variables|Default|GetTimerText) (Utilities|String|Append "0:0" (Utilities|String|ToString(Integer) (Math|Float|Ceil (Variables|Default|GettimeLeft)))))
      (else
        ;[1 1 1] If time left is greater than 10 seconds, display the value
        (Rendering|Components|TextRender|SetText (Variables|Default|GetTimerText) (Utilities|String|Append "0:" (Utilities|String|ToString(Integer) (Math|Float|Ceil (Variables|Default|GettimeLeft)))))))
    (elif (<= (Variables|Default|GettimeLeft) 0.0)
      ;[1 1 1] If the time is below 0, toggle blinking and change text
      (Variables|Default|SettimeLeft (- 1.0 (- 0.0 (Variables|Default|GettimeLeft))))
      (Variables|Default|SetblinkOn (not (Variables|Default|GetblinkOn)))
      (if (Variables|Default|GetblinkOn)
        (Rendering|Components|TextRender|SetText _timertext "0:00")
        (else
          (Rendering|Components|TextRender|SetText _timertext "     ")))
      (else
        ;[1 1 1] Decrement time left
        (Variables|Default|SettimeLeft (- (Variables|Default|GettimeLeft) DeltaSeconds))))))

(event EventBeginPlay
  (CallFunction|InitializeClock))

(fn ConstructionScript
  (if (Variables|LevelEditing|GetSnapToWall)
    (Rendering|SetVisibility (Variables|Default|GetArrowTowardsWall) true false)
    (Rendering|SetVisibility (Variables|Default|GetWallPlane) true false)
    (LevelEditing|SnaptoLevel)
    (else
      (Rendering|SetVisibility (Variables|Default|GetArrowTowardsWall) false false)
      (Rendering|SetVisibility (Variables|Default|GetWallPlane) false false))))

(fn ResetTimer
  (Variables|Default|SettimeLeft (Variables|Default|GetloopTime))
  (Variables|Default|SethasStarted true))

(fn InitializeClock
  (Rendering|Components|TextRender|SetText (Variables|Default|GetTimerText) "     ")
  (Variables|Default|SettimeLeft 1.0)
  (Variables|Default|SetblinkOn false)
  (Variables|Default|SethasStarted false))

(fn SnaptoLevel
  (LocalVariables|SetTowardsWall (* (Transformation|GetActorForwardVector) -1.0))
  (LocalVariables|SetCurrentLocation (+ (Transformation|GetActorLocation) (* (Math|Vector|Normalize (Transformation|GetActorForwardVector)) 4e+01)))
  (bind (_outhit _returnvalue) (Collision|LineTraceForObjects (LocalVariables|GetCurrentLocation) (+ (LocalVariables|GetCurrentLocation) (* (Math|Vector|Normalize (LocalVariables|GetTowardsWall)) 8e+01)) (Utilities|Array|MakeArray "ObjectTypeQuery2" "ObjectTypeQuery1") false 0 "None"))
  (if _returnvalue
    (Utilities|IsValid (.HitActor (Collision|BreakHitResult _outhit))
      (:Is%20Valid
        ;[1 1 1] Translate and rotate this object to snap to the wall or floor underneath it
        (Transformation|SetActorLocation (+ (.Location (Collision|BreakHitResult _outhit)) (* (Math|Vector|Normalize (* (.Normal (Collision|BreakHitResult _outhit)) 1.0)) 2.0)) false)
        (if (not (Math|Vector|Equal(Vector) (Math|Vector|Normalize (Math|Vector|GetUpVector (Math|Rotator|MakeRotfromZ (.Normal (Collision|BreakHitResult _outhit))))) (Math|Vector|Normalize (Transformation|GetActorForwardVector)) 0.001))
          (Transformation|SetActorRotation (Math|Rotator|MakeRotfromX (.Normal (Collision|BreakHitResult _outhit)))))))))