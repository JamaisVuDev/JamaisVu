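; Look-sensor actor that switches linked GlassDoor and Indicator objects on while it keeps receiving ActivateSensor calls.
; ActivateSensor sets a flag that Tick consumes, using CanTrigger to fire activation once and deactivation once the calls stop.
; Both events swap the sensor's material between green and red and forward the state to each object in ActivatableObjects.
; The construction script sizes the HitRadius capsule from MinLookSensorDistance.
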(event `self.ReceiveTick`
  (params (DeltaSeconds :type "Float (single-precision)"))
  (if (and (`self.sensorActivated`) (`self.canTrigger`))
    (`self.Activate Objects`)
    (set `self.canTrigger` false)
    (elif (`self.sensorActivated`)
      (set `self.sensorActivated` false)
      (elif (not (`self.canTrigger`))
        (`self.Deactivate Objects`)
        (set `self.canTrigger` true)))))

(event `Activate Objects`
  (`PrimitiveComponent.SetMaterial` (`self.lookSensorObject`) 1 "/Game/Materials/SensorGreenMaterial.SensorGreenMaterial")
  (for _array_element (`self.activatableObjects`)
    (bind _asglass_door (cast `/Game/Blueprints/GlassDoor` _array_element)
      (:`then`
        (`/Game/Blueprints/GlassDoor.Activate` _asglass_door))
      (:`CastFailed`
        (bind _asindicator (cast `/Game/Blueprints/Indicator` _array_element))
        (`/Game/Blueprints/Indicator.Activate` _asindicator)))))

(event `Deactivate Objects`
  (`PrimitiveComponent.SetMaterial` (`self.lookSensorObject`) 1 "/Game/Materials/SensorRedMaterial.SensorRedMaterial")
  (for _array_element (`self.activatableObjects`)
    (bind _asglass_door (cast `/Game/Blueprints/GlassDoor` _array_element)
      (:`then`
        (`/Game/Blueprints/GlassDoor.Deactivate` _asglass_door))
      (:`CastFailed`
        (bind _asindicator (cast `/Game/Blueprints/Indicator` _array_element))
        (`/Game/Blueprints/Indicator.Deactivate` _asindicator)))))

(fn `activateSensor`
  (set `self.sensorActivated` true))

(fn `UserConstructionScript`
  (`CapsuleComponent.SetCapsuleRadius` (`self.HitRadius`) (`self.minLookSensorDistance`) false))